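; Proximity-driven animated door that opens for the player's ThirdPersonCharacter only when its Door2check flag is set.
; Tick measures player distance each frame, calling DorrOpen inside a fixed radius with the flag set and DoorClosed outside it.
; Opening plays the skeletal mesh animation and disables Box collision; closing plays the reverse animation and restores it.
; Two DoOnce gates reset each other so each transition fires once.
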(event `DorrOpen`
  (`/Engine/EditorBlueprintResources/StandardMacros.DoOnce` false :!label _label
    (:`Completed`
      (`SkeletalMeshComponent.PlayAnimation` (`self.SkeletalMesh`) "/Game/Doors/NiceDoorsMate_1__Anim.NiceDoorsMate_1__Anim" false)
      (`PrimitiveComponent.SetCollisionEnabled` (`self.Box`) "NoCollision")
      (goto _label_2 :!via `Reset`))))

(event `DoorClosed`
  (`/Engine/EditorBlueprintResources/StandardMacros.DoOnce` false :!label _label_2
    (:`Completed`
      (`SkeletalMeshComponent.PlayAnimation` (`self.SkeletalMesh`) "/Game/Doors/NiceDoorsMate_1__Anim1reverse.NiceDoorsMate_1__Anim1reverse" false)
      (`PrimitiveComponent.SetCollisionEnabled` (`self.Box`) "QueryAndPhysics")
      (goto _label :!via `Reset`))))

(event `self.ReceiveTick`
  (params (DeltaSeconds :type "Float (single-precision)"))
  (`|ExecutionSequence`
    (:`then_0`
      (if (< (`KismetMathLibrary.VSize` (- (`self.K2_GetActorLocation` (`GameplayStatics.GetPlayerCharacter` 0)) (`self.K2_GetActorLocation`))) 225.0)
        (if (`/Game/ThirdPersonBP/Blueprints/ThirdPersonCharacter.Door2check` (stale _asthird_person_character))
          (`self.DorrOpen`))
        (else
          (`self.DoorClosed`))))
    (:`then_1`
      (bind _asthird_person_character (cast `/Game/ThirdPersonBP/Blueprints/ThirdPersonCharacter` (`GameplayStatics.GetPlayerCharacter` 0))))))

(fn `UserConstructionScript`)