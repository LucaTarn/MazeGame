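; Proximity-driven door that opens when the first player character comes near and closes when they move away.
; Tick measures the distance to the player and calls the open or close event against a fixed radius.
; Two cross-resetting DoOnce gates make the skeletal mesh play each one-shot animation only once per change, using a separate reversed animation for closing.
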(event `DorrOpen`
  (`/Engine/EditorBlueprintResources/StandardMacros.DoOnce` false :!label _label
    (:`Completed`
      (`SkeletalMeshComponent.PlayAnimation` (`self.SkeletalMesh`) "/Game/Doors/NiceDoorsMate_1__Anim.NiceDoorsMate_1__Anim" false)
      (goto _label_2 :!via `Reset`))))

(event `DoorClosed`
  (`/Engine/EditorBlueprintResources/StandardMacros.DoOnce` false :!label _label_2
    (:`Completed`
      (`SkeletalMeshComponent.PlayAnimation` (`self.SkeletalMesh`) "/Game/Doors/NiceDoorsMate_1__Anim1reverse.NiceDoorsMate_1__Anim1reverse" false)
      (goto _label :!via `Reset`))))

(event `self.ReceiveTick`
  (params (DeltaSeconds :type "Float (single-precision)"))
  (if (< (`KismetMathLibrary.VSize` (- (`self.K2_GetActorLocation` (`GameplayStatics.GetPlayerCharacter` 0)) (`self.K2_GetActorLocation`))) 225.0)
    (`self.DorrOpen`)
    (else
      (`self.DoorClosed`))))

(fn `UserConstructionScript`)